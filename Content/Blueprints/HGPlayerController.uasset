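; HGPlayerController is a player controller that turns axis input into movement and look for the controlled pawn.
; Move axes add movement input along the controller's own forward and right vectors, with forward flattened to the horizontal plane and normalized so pitch does not affect it.
; Look axes pass their values straight to the pawn as controller pitch and yaw input.
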(event Input|AxisEvents|InputAxisMoveHorizontally
  (params (AxisValue :type Float%20%28single-precision%29))
  ;[1 1 1] Ground Movement
  (Pawn|Input|AddMovementInput (Pawn|GetControlledPawn) (Transformation|GetActorRightVector) AxisValue false))

(event Input|AxisEvents|InputAxisLookHorizontally
  (params (AxisValue :type Float%20%28single-precision%29))
  ;[1 1 1] Looking Around
  (Pawn|Input|AddControllerYawInput (Pawn|GetControlledPawn) AxisValue))

(event Input|AxisEvents|InputAxisMoveVertically
  (params (AxisValue :type Float%20%28single-precision%29))
  (bind _returnvalue (Transformation|GetActorForwardVector))
  (bind (_x _y) (Math|Vector|BreakVector _returnvalue))
  ;[1 1 1] Ground Movement
  (Pawn|Input|AddMovementInput (Pawn|GetControlledPawn) (Math|Vector|Normalize (Math|Vector|MakeVector _x _y 0.0)) AxisValue false))

(event Input|AxisEvents|InputAxisLookVertically
  (params (AxisValue :type Float%20%28single-precision%29))
  ;[1 1 1] Looking Around
  (Pawn|Input|AddControllerPitchInput (Pawn|GetControlledPawn) AxisValue))

(fn ConstructionScript)